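; Level sequence Blueprint for an enemy wall burst moment in the horror blockouts, supplying that scare's impact effects.
; Its SpecialEvents event plays a shock camera shake and a punch-named sound at the actor's location.
; It also disables the player character's input for a half-second stun, then re-enables it via the first-person player controller.
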(event `self.Special Events`
  (`GameplayStatics.PlayWorldCameraShake` "/Game/RoguesNewContent/HorrorBlockouts/LevelSequences/SequenceAssets/BP_CamShake_Shock.BP_CamShake_Shock_C" (`self.K2_GetActorLocation`) 0.0 1000.0)
  (`GameplayStatics.PlaySoundAtLocation` "/Game/WalkingSim/Audio/Triggered/punch-a-rock-161647-_AudioTrimmer_com_.punch-a-rock-161647-_AudioTrimmer_com_" (`self.K2_GetActorLocation`) (struct) 1.0 1.0 0.0 null null null null)
  (bind _asbp_first_person_player_controller (cast `/Game/FirstPerson/Blueprints/BP_FirstPersonPlayerController` (`GameplayStatics.GetPlayerController` 0)))
  (`self.DisableInput` (`GameplayStatics.GetPlayerCharacter` 0) _asbp_first_person_player_controller)
  (`KismetSystemLibrary.Delay` 0.5)
  (bind _asbp_first_person_player_controller_2 (cast `/Game/FirstPerson/Blueprints/BP_FirstPersonPlayerController` (`GameplayStatics.GetPlayerController` 0)))
  (`self.EnableInput` (`GameplayStatics.GetPlayerCharacter` 0) _asbp_first_person_player_controller_2))

(fn `UserConstructionScript`
  (`parent.UserConstructionScript`))