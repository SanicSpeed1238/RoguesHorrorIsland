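; BP_PlatformSwitch is an interactable button that moves a referenced platform in the level.
; Interact calls MovePlatform on that reference, swaps the button to its active material, and plays a rumble sound and world camera shake at the switch.
; A flag blocks reuse during a short delay, then the inactive material returns.
; A box overlap shows the widget only while the switch is usable and hides it on exit.
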(event `self.ReceiveBeginPlay`
  (`SceneComponent.SetVisibility` (`self.Widget`) false false)
  (`PrimitiveComponent.SetMaterial` (`self.ButtonMesh`) 0 (`self.InactiveMaterial`)))

(event `self.Interact`
  (if (`self.CanInteract`)
    (`/Game/RoguesNewContent/HorrorBlockouts/LevelAssets/PlatformSwitch/BP_MovingPlatform.Move Platform` (`self.PlatformRef`))
    (`PrimitiveComponent.SetMaterial` (`self.ButtonMesh`) 0 (`self.ActiveMaterial`))
    (set `self.CanInteract` false)
    (`GameplayStatics.PlaySoundAtLocation` "/Game/RoguesNewContent/HorrorBlockouts/LevelAssets/PlatformSwitch/SND_PlatformRumble.SND_PlatformRumble" (`self.K2_GetActorLocation`) (struct) 1.0 1.0 0.0 null null null null)
    (`GameplayStatics.PlayWorldCameraShake` "/Game/RoguesNewContent/HorrorBlockouts/LevelAssets/PlatformSwitch/BP_CamShake_Platform.BP_CamShake_Platform_C" (`self.K2_GetActorLocation`) 0.0 1000.0)
    (`KismetSystemLibrary.Delay` 3.0)
    (`PrimitiveComponent.SetMaterial` (`self.ButtonMesh`) 0 (`self.InactiveMaterial`))
    (set `self.CanInteract` true)))

(event `self.Box.OnComponentBeginOverlap`
  (params (OverlappedComponent :type "PrimitiveComponent Object Reference") (OtherActor :type "Actor Object Reference") (OtherComp :type "PrimitiveComponent Object Reference") (OtherBodyIndex :type Integer) (bFromSweep :type Boolean) (SweepResult :type "HitResult Structure (by ref)"))
  (if (`self.CanInteract`)
    (`SceneComponent.SetVisibility` (`self.Widget`) true false)))

(event `self.Box.OnComponentEndOverlap`
  (params (OverlappedComponent :type "PrimitiveComponent Object Reference") (OtherActor :type "Actor Object Reference") (OtherComp :type "PrimitiveComponent Object Reference") (OtherBodyIndex :type Integer))
  (`SceneComponent.SetVisibility` (`self.Widget`) false false))

(fn `UserConstructionScript`)