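; BP_LevelSequenceTrigger is a trigger box that plays an assigned level sequence once when the horror first-person player character walks into it.
; On overlap it confirms the actor is the player pawn and calls SpecialEvents, which here only prints a debug message.
; If the sequence reference is valid, it creates a player for that asset, plays it and sets Triggered to block repeats.
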(event `self.Box.OnComponentBeginOverlap`
  (params (OverlappedComponent :type "PrimitiveComponent Object Reference") (OtherActor :type "Actor Object Reference") (OtherComp :type "PrimitiveComponent Object Reference") (OtherBodyIndex :type Integer) (bFromSweep :type Boolean) (SweepResult :type "HitResult Structure (by ref)"))
  (if (not (`self.triggered`))
    (bind _asbp_horror_first_person_character (cast `/Game/WalkingSim/Character/BP_Horror_FirstPersonCharacter` (`GameplayStatics.GetPlayerPawn` 0)))
    (if (== _asbp_horror_first_person_character OtherActor)
      (`self.Special Events`)
      (`/Engine/EditorBlueprintResources/StandardMacros.IsValid` (`self.LevelSequenceRef`)
        (:`Is Valid`
          (bind _outactor (`LevelSequencePlayer.CreateLevelSequencePlayer` (`LevelSequenceActor.LevelSequenceAsset` (`self.LevelSequenceRef`))))
          (`MovieSceneSequencePlayer.Play` (`LevelSequenceActor.SequencePlayer` _outactor))
          (set `self.triggered` true))))))

(event `Special Events`
  (`KismetSystemLibrary.PrintString` "Sequence Triggered!"))

(fn `UserConstructionScript`)