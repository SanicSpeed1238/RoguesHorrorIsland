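; BP_FallingTree is a level actor for a tree that topples once when its RotateTree event is called.
; A DoOnce gate starts PlatformTimeline, which lerps the TreeMesh relative rotation from the actor's rotation toward RotateDirection.
; Each timeline update also clears IsMoving, flips InitialState and recomputes target positions, which the rotation never uses.
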(event `self.ReceiveBeginPlay`
  (`self.Set Target Positions` (`self.initialState`)))

(event `Set Target Positions`
  (params (Initial :type Boolean))
  (set `self.InitialPosition` (`self.K2_GetActorLocation`))
  (if Initial
    (set `self.TargetPosition` (+ (`self.InitialPosition`) (`self.RotateDirection`)))
    (else
      (set `self.TargetPosition` (- (`self.InitialPosition`) (`self.RotateDirection`))))))

(event `Rotate Tree`
  (bind (_returnvalue_roll _returnvalue_pitch _returnvalue_yaw) (`KismetMathLibrary.BreakRotator` (`self.K2_GetActorRotation`)))
  (`/Engine/EditorBlueprintResources/StandardMacros.DoOnce` false
    (:`Completed`
      (if (not (`self.isMoving`))
        (set `self.isMoving` true)
        (bind (_direction _value) (`Timeline|Platform Timeline`)
          (:`Update`
            (`SceneComponent.K2_SetRelativeRotation` (`self.TreeMesh`) (`KismetMathLibrary.MakeRotator` (`KismetMathLibrary.Lerp` _returnvalue_roll (.x (`self.RotateDirection`)) _value) (`KismetMathLibrary.Lerp` _returnvalue_pitch (.y (`self.RotateDirection`)) _value) (`KismetMathLibrary.Lerp` _returnvalue_yaw (.z (`self.RotateDirection`)) _value)) false false)
            (set `self.isMoving` false)
            (bind _output_get (set `self.initialState` (not (`self.initialState`))))
            (`self.Set Target Positions` _output_get)))))))

(fn `UserConstructionScript`)